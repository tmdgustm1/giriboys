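; BP_CounterSwitch is a counting switch that starts and stops a set of actors each time its PressF event fires.
; Each press increments Count, wraps it to zero after nine, and shows it on a TextRender.
; Count parity then selects the state: odd runs the actors, even stops them.
; The state reaches every entry in the Actors array through DoPlayAndStop on the BPI_PlayStop interface.
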(event `/Game/FirstGame/BPI_Switch.PressF`
  (`|ExecutionSequence`
    (:`then_0`
      (`self.Count증가표시`))
    (:`then_1`
      (if (== (mod (`self.Count`) 2) 1)
        (`self.Actors가 동작하는상태`)
        (else
          (`self.Actor가 멈춰있는상태`))))))

(fn `Actors가 동작하는상태`
  ; Actors가 동작하는 상태
  (for _array_element (`self.Actors`)
    (bind _asbpi_play_stop (cast `/Game/FirstGame/BPI_PlayStop` _array_element))
    (`/Game/FirstGame/BPI_PlayStop.DoPlayAndStop` _asbpi_play_stop true)))

(fn `Actor가 멈춰있는상태`
  ; Actors가 멈춰있는 상태
  (for _array_element (`self.Actors`)
    (bind _asbpi_play_stop (cast `/Game/FirstGame/BPI_PlayStop` _array_element))
    (`/Game/FirstGame/BPI_PlayStop.DoPlayAndStop` _asbpi_play_stop false)))

(fn `Count1Up`
  ; Count를 1증가
  (set `self.Count` (+ (`self.Count`) 1)))

(fn `Count증가표시`
  ; Count 증가 표시
  (`self.Count1Up`)
  (`self.Over9Count0`)
  (`self.ShowCount`))

(fn `Over9Count0`
  ; Count가 9보다 크면
  (if (> (`self.Count`) 9)
    ; Count 0으로 변경
    (set `self.Count` 0)))

(fn `ShowCount`
  ; Count를 Text Rander에 표시
  (`TextRenderComponent.K2_SetText` (`self.TextRender`) (`KismetTextLibrary.Conv_IntToText` (`self.Count`))))

(fn `UserConstructionScript`)