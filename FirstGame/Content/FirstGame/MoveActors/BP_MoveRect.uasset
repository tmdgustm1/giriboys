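; BP_MoveRect is an actor that moves its Cube around a rectangular loop in the relative XZ plane while IsPlay is set.
; Tick runs a MoveType state machine (Right, Up, Left, Down), stepping a fixed distance per frame, independent of delta time, and switching at each boundary.
; DoPlay, DoStop and EventSwitchToggle control IsPlay.
; DoPlayAndStop ignores its input, always calling DoPlay and returning false.
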(event `self.ReceiveTick`
  (params (DeltaSeconds :type "Float (single-precision)"))
  (if (`self.IsPlay`)
    (switch `/Game/FirstGame/ENUM_MoveType` (`self.MoveType`)
      (:`NewEnumerator0`
        (set `self.X의 위치` (+ (`self.X의 위치`) 5.0))
        (`SceneComponent.K2_SetRelativeLocation` (`self.Cube`) (`KismetMathLibrary.MakeVector` (`self.X의 위치`) 0.0 (`self.Z의 위치`)) false false)
        (if (>= (`self.X의 위치`) 500.0)
          (set `self.MoveType` "NewEnumerator1")))
      (:`NewEnumerator1`
        (set `self.Z의 위치` (+ (`self.Z의 위치`) 5.0))
        (`SceneComponent.K2_SetRelativeLocation` (`self.Cube`) (`KismetMathLibrary.MakeVector` (`self.X의 위치`) 0.0 (`self.Z의 위치`)) false false)
        (if (>= (`self.Z의 위치`) 500.0)
          (set `self.MoveType` "NewEnumerator2")))
      (:`NewEnumerator2`
        (set `self.X의 위치` (- (`self.X의 위치`) 5.0))
        (`SceneComponent.K2_SetRelativeLocation` (`self.Cube`) (`KismetMathLibrary.MakeVector` (`self.X의 위치`) 0.0 (`self.Z의 위치`)) false false)
        (if (<= (`self.X의 위치`) 0.0)
          (set `self.MoveType` "NewEnumerator3")))
      (:`NewEnumerator3`
        (set `self.Z의 위치` (- (`self.Z의 위치`) 5.0))
        (`SceneComponent.K2_SetRelativeLocation` (`self.Cube`) (`KismetMathLibrary.MakeVector` (`self.X의 위치`) 0.0 (`self.Z의 위치`)) false false)
        (if (<= (`self.Z의 위치`) 0.0)
          (set `self.MoveType` "NewEnumerator0"))))))

(event `DoPlay`
  (set `self.IsPlay` true))

(event `DoStop`
  (set `self.IsPlay` false))

(event `self.ReceiveBeginPlay`)

(fn `DoPlayAndStop`
  (params (IsPlay :type Boolean))
  (returns (bResult :type Boolean))
  (if true
    (`self.DoPlay`)
    (else
      (`self.DoStop`)))
  (return false))

(fn `EventSwitchToggle`
  (params (Toggle :type Boolean))
  (set `self.IsPlay` Toggle))

(fn `UserConstructionScript`)