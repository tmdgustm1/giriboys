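; Actor that moves its Cube back and forth on a timeline, with motion that can be started and stopped.
; Each timeline update scales a fixed offset vector to set the cube's relative location, without sweep.
; ISRight selects forward or reverse playback and flips on finish, looping the motion until DoStop halts it.
; DoPlayAndStop maps a boolean to DoPlay or DoStop and always returns false.
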(event `DoPlay`
  (if (`self.ISRight`) :!label _label
    (bind (_direction _value) (`Timeline|타임라인` :`NewTime` 0.5 :!label _label_2)
      (:`Update`
        (`SceneComponent.K2_SetRelativeLocation` (`self.Cube`) (* _value (400.0 50.0 70.0)) false false))
      (:`Finished`
        (set `self.ISRight` (not (`self.ISRight`)))
        (goto _label)))
    (else
      (goto _label_2 :!via `Reverse`))))

(event `DoStop`
  (goto _label_2 :!via `Stop`))

(fn `DoPlayAndStop`
  (params (IsPlay :type Boolean))
  (returns (bResult :type Boolean))
  (if IsPlay
    (`self.DoPlay`)
    (else
      (`self.DoStop`)))
  (return false))

(fn `UserConstructionScript`)