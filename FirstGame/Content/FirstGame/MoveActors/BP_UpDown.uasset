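; BP_UpDown is an actor that bobs its StaticMesh up and down while playback is enabled.
; On Tick it steps LocZ by a fixed amount and sets the mesh's relative Z, flipping IsMoveUp at the top and bottom limits, so speed depends on frame rate.
; DoPlay and DoStop toggle the ISPlay flag, and DoPlayAndStop routes a boolean to either event, always returning false.
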(event `self.ReceiveTick`
  (params (DeltaSeconds :type "Float (single-precision)"))
  (if (`self.ISPlay`)
    (if (`self.IsMoveUp`)
      (set `self.LocZ` (+ (`self.LocZ`) 5.0))
      (`SceneComponent.K2_SetRelativeLocation` (`self.StaticMesh`) (`KismetMathLibrary.MakeVector` 0.0 0.0 (`self.LocZ`)) false false)
      (if (>= (`self.LocZ`) 500.0)
        (set `self.IsMoveUp` false))
      (else
        (set `self.LocZ` (- (`self.LocZ`) 5.0))
        (`SceneComponent.K2_SetRelativeLocation` (`self.StaticMesh`) (`KismetMathLibrary.MakeVector` 0.0 0.0 (`self.LocZ`)) false false)
        (if (<= (`self.LocZ`) 0.0)
          (set `self.IsMoveUp` true))))))

(event `DoPlay`
  (set `self.ISPlay` true))

(event `DoStop`
  (set `self.ISPlay` false))

(fn `DoPlayAndStop`
  (params (IsPlay :type Boolean))
  (returns (bResult :type Boolean))
  (if IsPlay
    (`self.DoPlay`)
    (else
      (`self.DoStop`)))
  (return false))

(fn `UserConstructionScript`)