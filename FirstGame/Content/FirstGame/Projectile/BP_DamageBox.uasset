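; BP_DamageBox is an actor that acts as a repeating explosion hazard at its own location.
; BeginPlay starts a looping timer that calls DoExplosion every second.
; Each blast spawns a scaled-up explosion emitter, applies radial damage that ignores itself, and applies a strong constant-falloff radial impulse to its Sphere component.
; A red debug sphere shows the shared blast radius for a second.
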(event `self.ReceiveBeginPlay`
  (`KismetSystemLibrary.K2_SetTimer` null "DoExplosion" 1.0 true))

(fn `DoExplosion`
  (bind (_returnvalue_location _returnvalue_rotation) (`KismetMathLibrary.BreakTransform` (`self.GetTransform`)))
  (`GameplayStatics.SpawnEmitterAtLocation` "/Game/StarterContent/Particles/P_Explosion.P_Explosion" _returnvalue_location _returnvalue_rotation (3.0 3.0 3.0))
  (`GameplayStatics.ApplyRadialDamage` 1.0 (`self.K2_GetActorLocation`) 500.0 null (`|MakeArray` self :!type "Actor Object Reference") self null)
  (`PhysicsObjectBlueprintLibrary.ApplyRadialImpulse` (`self.Sphere`) (`self.K2_GetActorLocation`) 500.0 5000000.0 "RIF_Constant")
  (`KismetSystemLibrary.DrawDebugSphere` (`self.K2_GetActorLocation`) 500.0 12 (struct :`R` 1.0 :`B` 0.060372 :`A` 1.0) 1.0 1.0))

(fn `UserConstructionScript`)