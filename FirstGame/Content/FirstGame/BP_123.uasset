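; BP_123 is an actor that moves its Cube component along an axis-aligned path, stepped every Tick.
; An enum state, NewVar, selects the direction: Left lowers X축 to a limit, then switches to Up, which raises Z축.
; Up tests X축 rather than Z축 for its switch to Right, so that switch is not reached after Left.
; Right has no movement logic.
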(event `self.ReceiveTick`
  (params (DeltaSeconds :type "Float (single-precision)"))
  (switch `/Game/FirstGame/ENUM_123` (`self.NewVar`)
    (:`NewEnumerator0`
      (bind _output_get (set `self.X축` (- (`self.X축`) 5.0)))
      (`SceneComponent.K2_SetRelativeLocation` (`self.Cube`) (`KismetMathLibrary.MakeVector` _output_get 0.0 (`self.z축`)) false false)
      (if (<= (`self.X축`) -300.0)
        (set `self.NewVar` "NewEnumerator1")))
    (:`NewEnumerator1`
      (bind _output_get_2 (set `self.z축` (+ (`self.z축`) 5.0)))
      (`SceneComponent.K2_SetRelativeLocation` (`self.Cube`) (`KismetMathLibrary.MakeVector` (`self.X축`) 0.0 _output_get_2) false false)
      (if (>= (`self.X축`) 300.0)
        (set `self.NewVar` "NewEnumerator2")))))

(fn `UserConstructionScript`)