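; BP_Counter is an actor with a widget component that displays a counter.
; Each tick it rotates the widget to face the player camera.
; Pressing F increments Count, wraps it to zero after 9, and pushes the value to CountWidget.
; DoPlay and DoStop reset Count to zero without refreshing the widget.
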(event `self.ReceiveTick`
  (params (DeltaSeconds :type "Float (single-precision)"))
  (`SceneComponent.K2_SetWorldRotation` (`self.Widget`) (`KismetMathLibrary.FindLookAtRotation` (`SceneComponent.K2_GetComponentLocation` (`self.Widget`)) (`self.K2_GetActorLocation` (`GameplayStatics.GetPlayerCameraManager` 0))) false false))

(event `/Game/FirstGame/BPI_Switch.PressF`
  (`self.UpdateCount`)
  (bind _ascount_widget (cast `/Game/FirstGame/Widget/CountWidget` (`WidgetComponent.GetUserWidgetObject` (`self.Widget`))))
  (`/Game/FirstGame/Widget/CountWidget.UpdateCount` _ascount_widget (`self.Count`)))

(event `DoPlay`
  (set `self.Count` 0))

(event `DoStop`
  (set `self.Count` 0))

(fn `UpdateCount`
  ; Count를 1증가
  (set `self.Count` (+ (`self.Count`) 1))
  ; Count가 9보다 크면
  (if (> (`self.Count`) 9)
    ; Count 0으로 변경
    (set `self.Count` 0)))

(fn `UserConstructionScript`)