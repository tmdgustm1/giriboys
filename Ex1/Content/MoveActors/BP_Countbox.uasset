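; BP_Countbox is a counter box that counts overlaps on its Cube and shows a number on a text render.
; Each overlap increments Count, wraps it to zero once it passes nine, and displays Count minus nine, so the shown value is zero or negative.
; DoPlay and DoStop both reset Count without refreshing the text.
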(event `self.Cube.OnComponentBeginOverlap`
  (params (OverlappedComponent :type "PrimitiveComponent Object Reference") (OtherActor :type "Actor Object Reference") (OtherComp :type "PrimitiveComponent Object Reference") (OtherBodyIndex :type Integer) (bFromSweep :type Boolean) (SweepResult :type "HitResult Structure (by ref)"))
  (set `self.Count` (+ (`self.Count`) 1))
  (if (> (`self.Count`) 9)
    (set `self.Count` 0))
  (`TextRenderComponent.K2_SetText` (`self.TextRender`) (`KismetTextLibrary.Conv_IntToText` (- (`self.Count`) 9))))

(event `DoPlay`
  (set `self.Count` 0))

(event `DoStop`
  (set `self.Count` 0))

(fn `UserConstructionScript`)