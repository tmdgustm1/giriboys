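; BP_LeftRight is an actor that slides its Cube component back and forth along the relative X axis while IsPlay is true.
; Each Tick shifts a stored X position by a fixed step and applies it as the Cube's relative location.
; A direction boolean flips at the 0 and 500 bounds.
; The step ignores delta time, so speed depends on frame rate.
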(event `self.ReceiveTick`
  (params (DeltaSeconds :type "Float (single-precision)"))
  (if (`self.IsPlay`)
    (if (`self.오른쪽 이동인가?`)
      ; X에 위치에 100을 더한다.
      (bind _output_get (set `self.X의위치` (+ (`self.X의위치`) 5.0)))
      ; Box에 상대좌표 x를 "X의 위치" 값으로 변경한다
      ;; 구조체의 값을 각각의 수치로 분할할 수 있다
      (`SceneComponent.K2_SetRelativeLocation` (`self.Cube`) (`KismetMathLibrary.MakeVector` _output_get) false false)
      (if (>= (`self.X의위치`) 500.0)
        (set `self.오른쪽 이동인가?` false))
      (else
        (bind _output_get_2 (set `self.X의위치` (- (`self.X의위치`) 5.0)))
        (`SceneComponent.K2_SetRelativeLocation` (`self.Cube`) (`KismetMathLibrary.MakeVector` _output_get_2) false false)
        (if (<= (`self.X의위치`) 0.0)
          (set `self.오른쪽 이동인가?` true))))))

(fn `UserConstructionScript`)