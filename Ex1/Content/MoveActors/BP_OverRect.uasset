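; BP_OverRect is an actor that moves its Cube component around a square loop in the local XZ plane.
; Each Tick while IsPlay is set, a MoveType state switch steps the X or Z position by a fixed amount, ignoring delta time, and advances to the next side at each corner.
; DoPlay and DoStop events start and pause the motion.
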(event `self.ReceiveBeginPlay`)

(event `self.ReceiveTick`
  (params (DeltaSeconds :type "Float (single-precision)"))
  (if (`self.IsPlay`)
    (switch `/Game/MoveActors/Enum_MoveType` (`self.MoveType`)
      (:`NewEnumerator0`
        (set `self.X의위치` (+ (`self.X의위치`) 5.0))
        (`SceneComponent.K2_SetRelativeLocation` (`self.Cube`) (`KismetMathLibrary.MakeVector` (`self.X의위치`) 0.0 (`self.Z의위치`)) false false)
        (if (>= (`self.X의위치`) 500.0)
          (set `self.MoveType` "NewEnumerator1")))
      (:`NewEnumerator1`
        (set `self.Z의위치` (+ (`self.Z의위치`) 5.0))
        (`SceneComponent.K2_SetRelativeLocation` (`self.Cube`) (`KismetMathLibrary.MakeVector` (`self.X의위치`) 0.0 (`self.Z의위치`)) false false)
        (if (>= (`self.Z의위치`) 500.0)
          (set `self.MoveType` "NewEnumerator2")))
      (:`NewEnumerator2`
        (set `self.X의위치` (- (`self.X의위치`) 5.0))
        (`SceneComponent.K2_SetRelativeLocation` (`self.Cube`) (`KismetMathLibrary.MakeVector` (`self.X의위치`) 0.0 (`self.Z의위치`)) false false)
        (if (<= (`self.X의위치`) 0.0)
          (set `self.MoveType` "NewEnumerator3")))
      (:`NewEnumerator3`
        (set `self.Z의위치` (- (`self.Z의위치`) 5.0))
        (`SceneComponent.K2_SetRelativeLocation` (`self.Cube`) (`KismetMathLibrary.MakeVector` (`self.X의위치`) 0.0 (`self.Z의위치`)) false false)
        (if (<= (`self.Z의위치`) 0.0)
          (set `self.MoveType` "NewEnumerator0"))))))

(event `DoPlay`
  (set `self.IsPlay` true))

(event `DoStop`
  (set `self.IsPlay` false))

(fn `UserConstructionScript`)