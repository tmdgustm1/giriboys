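; BP_SpawnerBase is a spawner that repeatedly drops a configurable SpawnClass actor into the level.
; BeginPlay starts a short looping timer bound to SpawnProjectile and stores its handle.
; Each tick of that timer spawns the actor at a random world X within SpawnRange and at SpawnHeight on Z, independent of the spawner's location.
; StopTimer clears and invalidates the handle to end spawning.
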(event `self.ReceiveBeginPlay`
  (bind _returnvalue (`KismetSystemLibrary.K2_SetTimerDelegate` (delegate `Spawn Projectile`) 0.2 true))
  (set `self.TimeHandler` _returnvalue))

(event `Spawn Projectile`
  (bind (_x _y) (`KismetMathLibrary.BreakVector2D` (`self.SpawnRange`)))
  (`|SpawnActorFromClass` (`self.Spawn Class`) (`KismetMathLibrary.MakeTransform` (`KismetMathLibrary.MakeVector` (`KismetMathLibrary.RandomFloatInRange` _x _y) 0.0 (`self.SpawnHeight`))) "Undefined" "MultiplyWithRoot" null null))

(event `Stop Timer`
  (`KismetSystemLibrary.K2_ClearAndInvalidateTimerHandle` (`self.TimeHandler`)))

(fn `UserConstructionScript`)