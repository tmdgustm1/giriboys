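; BP_PortalPassward is a password puzzle that reveals a Sphere when a set of counter objects shows the correct code.
; BeginPlay hides the Sphere and binds an event to the click dispatcher of each object in Counts, apparently FuncPressFClick.
; That handler prints a debug string and sets Sphere visibility from IsAllBox9.
; IsAllBox9 compares each Count to the Password entry at the same index, despite its name.
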(event `self.ReceiveBeginPlay`
  (`SceneComponent.SetVisibility` (`self.Sphere`) false false)
  (for _array_element (`self.Counts`)
    (add `/Game/BluePrintEx/BP_Counting.EventDispatcer_FClick` _array_element (`|CreateDelegate` :!event `FuncPressFClick`))))

(fn `FuncPressFClick`
  (`KismetSystemLibrary.PrintString` "Hello")
  (`SceneComponent.SetVisibility` (`self.Sphere`) (`self.IsAllBox9`) false))

(fn `IsAllBox9`
  (returns (AllBox9 :type Boolean))
  (for (_array_element _array_index) (`self.Counts`)
    (if (not (== (`/Game/BluePrintEx/BP_Counting.Count` _array_element) (`|GetArrayItem` (`self.Password`) _array_index)))
      (return false)))
  (return true))

(fn `UserConstructionScript`)